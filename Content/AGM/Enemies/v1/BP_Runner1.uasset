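; BP_Runner1 is a runner enemy character that shuttles back and forth between two goal points.
; A looping timer plays or reverses a Timeline that sweeps the actor between them, flipping the Reach flag near each end.
; A hit from an Ice-tagged actor calls HitbyIce and sets Freeze for a few seconds, which suspends those timer commands without stopping the Timeline.
; UpdateWalkSpeed sets the movement component's max walk speed.
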(event Custom|CustomEvent_0
  (if (not (Variables|Default|GetFreeze))
    (if (Variables|Default|Getreach)
      (bind _newtrack_0 (Timeline|Timeline Play)
        (:Update
          (Transformation|SetActorLocation (Math|Vector|Lerp(Vector) (Variables|Default|GetGoal_0) (Variables|Default|GetGoal) _newtrack_0) true false)
          (if (Variables|Default|Getreach)
            (if (Utilities|Operators|EqualEqual (Transformation|GetActorLocation) (Variables|Default|GetGoal) 1e+01)
              (Variables|Default|Setreach false))
            (elif (Utilities|Operators|EqualEqual (Transformation|GetActorLocation) (Variables|Default|GetGoal_0) 1e+01)
              (Variables|Default|Setreach true)))))
      (else
        (Timeline|Timeline Reverse)))))

(event Custom|CustomEvent
  (Variables|Default|SetFreeze false))

(event EventTick
  (params (DeltaSeconds :type Float%20%28single-precision%29)))

(event Collision|EventHit
  (params (MyComp :type Primitive%20Component%20Object%20Reference) (Other :type Actor%20Object%20Reference) (OtherComp :type Primitive%20Component%20Object%20Reference) (bSelfMoved :type Boolean) (HitLocation :type Vector :default "0, 0, 0") (HitNormal :type Vector :default "0, 0, 0") (NormalImpulse :type Vector :default "0, 0, 0") (Hit :type Hit%20Result%20Structure%20%28by%20ref%29))
  (if (Actor|ActorHasTag Other "Ice")
    (Variables|Default|SetFreeze true)
    (Utilities|Time|SetTimerbyEvent (delegate Custom|CustomEvent) 3.0)
    (Default|CallHitbyIce)))

(event EventBeginPlay
  (bind _asbp_runner_controller (Utilities|Casting|CastToBP_RunnerController (Pawn|GetController)))
  (Variables|Default|SetAs%20BP%20Runner%20Controller _asbp_runner_controller)
  (Utilities|Time|SetTimerbyEvent (delegate Custom|CustomEvent_0) 0.1 true))

(fn ConstructionScript)

(fn UpdateWalkSpeed
  (params (Speed :type Float%20%28double-precision%29))
  (Variables|/Script/Engine.CharacterMovementComponent|SetMaxWalkSpeed (Variables|Character|GetCharacterMovement) Speed))