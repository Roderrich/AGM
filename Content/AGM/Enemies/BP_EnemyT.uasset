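; BP_EnemyT is an enemy that walks to a goal on BeginPlay and tracks its own health.
; Lethal damage fires the OnDeath dispatcher, whose bound handler moves the "Tagged" actor tag from the damage causer to this enemy.
; An Ice-tag hit check leads nowhere, and the timed freeze and speed-restore nodes are disconnected.
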(event Custom|OnDeath_Event
  (params (DamageCauser :type Object%20Object%20Reference) (DamagedPlayer :type Object%20Object%20Reference))
  (for _array_element (Variables|/Script/Engine.Actor|GetTags (Variables|Default|GetDamage%20Causer))
    (if (== _array_element "Tagged")
      (Utilities|Array|RemoveItem (Variables|/Script/Engine.Actor|GetTags (Variables|Default|GetDamage%20Causer)) "Tagged")
      (Utilities|Array|Add (Variables|Actor|GetTags) "Tagged"))))

(event Custom|CustomEvent)

(event EventBeginPlay
  (EventDispatchers|BindEventtoOnDeath (delegate Custom|OnDeath_Event))
  (AI|Navigation|SimpleMovetoLocation 0 (Variables|Default|GetGoal)))

(event Collision|EventHit
  (params (MyComp :type Primitive%20Component%20Object%20Reference) (Other :type Actor%20Object%20Reference) (OtherComp :type Primitive%20Component%20Object%20Reference) (bSelfMoved :type Boolean) (HitLocation :type Vector :default "0, 0, 0") (HitNormal :type Vector :default "0, 0, 0") (NormalImpulse :type Vector :default "0, 0, 0") (Hit :type Hit%20Result%20Structure%20%28by%20ref%29))
  (if (Actor|ActorHasTag Other "Ice")
    _))

(event Collision|EventActorBeginOverlap
  (params (OtherActor :type Actor%20Object%20Reference)))

(event Game|Damage|EventAnyDamage
  (params (Damage :type Float%20%28single-precision%29) (DamageType :type Damage%20Type%20Object%20Reference) (InstigatedBy :type Controller%20Object%20Reference) (DamageCauser :type Actor%20Object%20Reference))
  (bind _self self)
  (Variables|Default|SetDamage%20Causer DamageCauser)
  (if (<= (- (Variables|Default|GetCurrentHealth) Damage) 0.0)
    (Default|CallOnDeath _self (Variables|Default|GetDamage%20Causer) _self)
    (else
      (Variables|Default|SetCurrentHealth (- (Variables|Default|GetCurrentHealth) Damage)))))

(fn ConstructionScript)