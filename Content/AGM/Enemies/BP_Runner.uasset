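; BP_Runner is a character that the player wins against by touching: a Sphere overlap with BP_FirstPersonCharacter calls Win on that player.
; BeginPlay caches its BP_RunnerController, and UpdateWalkSpeed exposes the movement component's max walk speed.
; Movement logic is not in this graph: PawnSensing handlers and Tick are empty, and a forward SimpleMoveToLocation call is left unconnected.
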(event OnSeePawn(PawnSensing)
  (params (Pawn :type Pawn%20Object%20Reference)))

(event OnHearNoise(PawnSensing)
  (params (Instigator :type Pawn%20Object%20Reference) (Location :type Vector%20%28by%20ref%29 :default "0, 0, 0") (Volume :type Float%20%28single-precision%29)))

(event OnComponentBeginOverlap(Sphere)
  (params (OverlappedComponent :type Primitive%20Component%20Object%20Reference) (OtherActor :type Actor%20Object%20Reference) (OtherComp :type Primitive%20Component%20Object%20Reference) (OtherBodyIndex :type Integer) (bFromSweep :type Boolean) (SweepResult :type Hit%20Result%20Structure%20%28by%20ref%29))
  (bind _asplayer (Utilities|Casting|CastToBP_FirstPersonCharacter OtherActor))
  (Default|Win _asplayer))

(event EventTick
  (params (DeltaSeconds :type Float%20%28single-precision%29)))

(event EventBeginPlay
  (bind _asbp_runner_controller (Utilities|Casting|CastToBP_RunnerController (Pawn|GetController)))
  (Variables|Default|SetAs%20BP%20Runner%20Controller _asbp_runner_controller))

(fn ConstructionScript)

(fn UpdateWalkSpeed
  (params (Speed :type Float%20%28double-precision%29))
  (Variables|/Script/Engine.CharacterMovementComponent|SetMaxWalkSpeed (Variables|Character|GetCharacterMovement) Speed))