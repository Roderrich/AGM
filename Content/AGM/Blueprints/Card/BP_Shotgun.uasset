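; BP_Shotgun is a card Blueprint that, despite its asset name, presents itself as "Dash" and gives the player a dash ability.
; Activating it spends one ammo from the weapon component, updates the widget and triggers the dash component along the first-person camera's forward vector.
; The use that empties the ammo also starts the cooldown timer, and further activations during cooldown only print a warning.
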(event Custom|Dash
  (if (Variables|Default|GetCardCooldown)
    (Development|PrintString "Card on Cooldown" true true "(R=1.000000,G=0.052997,B=0.000000,A=1.000000)")
    (else
      (bind _output_get (Variables|/Game/AGM/Blueprints/Components/BPC_Weapon.BPC_Weapon_C|SetCurrentAmmo (Variables|Default|GetBPC_Weapon) (- (Variables|/Game/AGM/Blueprints/Components/BPC_Weapon.BPC_Weapon_C|GetCurrentAmmo (Variables|Default|GetBPC_Weapon)) 1)))
      (if (== _output_get 0)
        (Class|BPIWidget|UpdateWidget(Message) (Variables|Default|GetWidgetRef) _output_get)
        (Default|ActivateAbility (Variables|Default|GetBPC_Dash) (Math|Vector|GetForwardVector (Variables|/Game/FirstPerson/Blueprints/BP_FirstPersonCharacter.BP_FirstPersonCharacter_C|GetFirstPersonCamera (Variables|Default|GetPlayer_0))) (Variables|Default|GetPlayer_0))
        (CallFunction|CooldownTimer)
        (Variables|Default|SetCardCooldown true)
        (else
          (Class|BPIWidget|UpdateWidget(Message) (Variables|Default|GetWidgetRef) _output_get)
          (Default|ActivateAbility (Variables|Default|GetBPC_Dash) (Math|Vector|GetForwardVector (Variables|/Game/FirstPerson/Blueprints/BP_FirstPersonCharacter.BP_FirstPersonCharacter_C|GetFirstPersonCamera (Variables|Default|GetPlayer_0))) (Variables|Default|GetPlayer_0)))))))

(event EventBeginPlay
  (|CallParentFunction)
  (Variables|Default|SetIn%20Color%20and%20Opacity "(R=1.000000,G=1.000000,B=1.000000,A=1.000000)")
  (Variables|Default|SetTexture "/Game/AGM/Materials/Textures/fire-dash.fire-dash")
  (Variables|Default|SetName "Dash"))

(event Collision|EventActorBeginOverlap
  (params (OtherActor :type Actor%20Object%20Reference))
  (|CallParentFunction OtherActor) ; This node is disabled and will not be called.\nDrag off pins to build functionality.
)

(event EventTick
  (params (DeltaSeconds :type Float%20%28single-precision%29))
  (|CallParentFunction DeltaSeconds) ; This node is disabled and will not be called.\nDrag off pins to build functionality.
)

(event EventActivateAbility
  (CallFunction|Dash))

(fn ConstructionScript
  (|CallParentFunction))