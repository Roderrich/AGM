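; Assault rifle card ability: each activation spends one round from the weapon component and updates the card widget's ammo message.
; Firing traces from the first-person camera, then activates the freeze component with a transform ahead of the player, rotated toward the hit point.
; The last round starts the card cooldown, which blocks further use with an on-screen print.
; An unconnected copy of the firing logic remains in the EventGraph.
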(event EventBeginPlay
  (|CallParentFunction)
  (Variables|Default|SetIn%20Color%20and%20Opacity "(R=1.000000,G=1.000000,B=1.000000,A=1.000000)"))

(event Collision|EventActorBeginOverlap
  (params (OtherActor :type Actor%20Object%20Reference))
  (|CallParentFunction OtherActor) ; This node is disabled and will not be called.\nDrag off pins to build functionality.
)

(event EventTick
  (params (DeltaSeconds :type Float%20%28single-precision%29))
  (|CallParentFunction DeltaSeconds) ; This node is disabled and will not be called.\nDrag off pins to build functionality.
)

(event EventActivateAbility
  (if (Variables|Default|GetCardCooldown)
    (Development|PrintString "Card on Cooldown" true true "(R=1.000000,G=0.052997,B=0.000000,A=1.000000)")
    (else
      (bind _output_get (Variables|/Game/AGM/Blueprints/Components/BPC_Weapon.BPC_Weapon_C|SetCurrentAmmo (Variables|Default|GetBPC_Weapon) (- (Variables|/Game/AGM/Blueprints/Components/BPC_Weapon.BPC_Weapon_C|GetCurrentAmmo (Variables|Default|GetBPC_Weapon)) 1)))
      (if (== _output_get 0)
        (Class|BPIWidget|UpdateWidget(Message) (Variables|Default|GetWidgetRef) _output_get)
        (CallFunction|Ability)
        (CallFunction|CooldownTimer)
        (Variables|Default|SetCardCooldown true)
        (else
          (Class|BPIWidget|UpdateWidget(Message) (Variables|Default|GetWidgetRef) _output_get)
          (CallFunction|Ability))))))

(fn ConstructionScript
  (|CallParentFunction))

(fn Ability
  (bind _as_player (Variables|Default|GetAs%20Player))
  (bind _as_player_2 (Variables|Default|GetAs%20Player))
  (bind _firstpersoncamera (Variables|/Game/FirstPerson/Blueprints/BP_FirstPersonCharacter.BP_FirstPersonCharacter_C|GetFirstPersonCamera _as_player_2))
  (bind _rootcomponent (Variables|/Script/Engine.Actor|GetRootComponent _as_player))
  (bind _returnvalue (Transformation|GetWorldLocation _firstpersoncamera))
  (bind _returnvalue_2 (Transformation|GetWorldLocation _rootcomponent))
  (bind _outhit (Collision|LineTraceByChannel _returnvalue (+ _returnvalue (* (Math|Vector|GetForwardVector _firstpersoncamera) 1e+04)) "TraceTypeQuery1" false 0 "ForDuration"))
  (Default|ActivateAbility (Variables|Default|GetBPC_Freeze) (Math|Transform|MakeTransform (+ _returnvalue_2 (* (Math|Vector|GetForwardVector (Variables|/Game/FirstPerson/Blueprints/BP_FirstPersonCharacter.BP_FirstPersonCharacter_C|GetFirstPersonCamera _as_player)) 1e+02)) (Math|Rotator|FindLookatRotation _returnvalue_2 (.Location (Collision|BreakHitResult _outhit))))))