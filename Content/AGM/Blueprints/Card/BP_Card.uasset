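; BP_Card is a weapon card pickup that shows a WBP_Cards widget with ammo from its BPCWeapon component.
; On overlap, the first-person character registers and focuses the card, which snaps to the InFocusSocket on that character's mesh.
; A timer-driven cooldown reloads the weapon and refreshes the widget.
; Fire, stop-fire and ability events are empty, leaving the trigger and ammo-check logic disconnected, and GetID returns zero.
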(event OnComponentBeginOverlap(Box)
  (params (OverlappedComponent :type Primitive%20Component%20Object%20Reference) (OtherActor :type Actor%20Object%20Reference) (OtherComp :type Primitive%20Component%20Object%20Reference) (OtherBodyIndex :type Integer) (bFromSweep :type Boolean) (SweepResult :type Hit%20Result%20Structure%20%28by%20ref%29))
  (bind _self self)
  (Collision|SetCollisionEnabled (Variables|Default|GetBox) "NoCollision")
  (bind _asplayer (Utilities|Casting|CastToBP_FirstPersonCharacter OtherActor))
  (Class|BPIPlayer|AddCard(Message) _asplayer _self)
  (Default|Focus _asplayer _self)
  (bind _output_get (Variables|Default|SetAs%20Player _asplayer))
  (Transformation|AttachComponentToComponent (Variables|/Game/FirstPerson/Blueprints/BP_FirstPersonCharacter.BP_FirstPersonCharacter_C|GetFirstPersonMesh _output_get) "InFocusSocket" "SnapToTarget" "SnapToTarget" "SnapToTarget" true))

(event Custom|CooldownTimer
  (Utilities|Time|SetTimerbyEvent (delegate Custom|Cooldown) (Variables|/Game/AGM/Blueprints/Components/BPC_Weapon.BPC_Weapon_C|GetCooldown (Variables|Default|GetBPC_Weapon))))

(event Custom|Cooldown
  (Variables|Default|SetCardCooldown false)
  (Default|Reload (Variables|Default|GetBPC_Weapon))
  (Class|BPIWidget|UpdateWidget(Message) (Variables|Default|GetWidgetRef) (Variables|/Game/AGM/Blueprints/Components/BPC_Weapon.BPC_Weapon_C|GetMaxAmmo (Variables|Default|GetBPC_Weapon))))

(event EventActivateAbility)

(event Collision|EventActorBeginOverlap
  (params (OtherActor :type Actor%20Object%20Reference)))

(event EventTick
  (params (DeltaSeconds :type Float%20%28single-precision%29)))

(event EventBeginPlay
  (bind _returnvalue (UserInterface|CreateWidget "/Game/AGM/UI/WBP_Cards.WBP_Cards_C" 0 (Variables|Default|GetIn%20Color%20and%20Opacity) (Variables|/Game/AGM/Blueprints/Components/BPC_Weapon.BPC_Weapon_C|GetMaxAmmo (Variables|Default|GetBPC_Weapon))))
  (bind _output_get (Variables|Default|SetWidgetRef _returnvalue))
  (UserInterface|SetWidget (Variables|Default|GetWidget) _output_get)
  (Variables|/Game/AGM/UI/WBP_Cards.WBP_Cards_C|SetUseLeft (Variables|Default|GetWidgetRef) (Utilities|Text|ToText(Integer) (Variables|/Game/AGM/Blueprints/Components/BPC_Weapon.BPC_Weapon_C|GetCurrentAmmo (Variables|Default|GetBPC_Weapon)))))

(event EventFireWeapon)

(event EventStopFireWeapon)

(fn ConstructionScript)

(fn GetID
  (bind _defaultsceneroot (Variables|Default|GetDefaultSceneRoot))
  (bind _returnvalue (Transformation|GetRelativeTransform _defaultsceneroot))
  (bind (_x _y _z) (Math|Vector|BreakVector (.location _returnvalue)))
  (Transformation|SetRelativeTransform _defaultsceneroot (Math|Transform|MakeTransform (Math|Vector|MakeVector 0.0 _y _z) "0, 0, 0" "1.000000,1.000000,1.000000") false false)
  (return 0))