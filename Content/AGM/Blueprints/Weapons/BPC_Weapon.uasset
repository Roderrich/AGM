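; Weapon component for the first-person character that handles hitscan shooting.
; On BeginPlay it caches the owning character and its player controller, then adds the weapons Enhanced Input mapping context.
; The shoot action line-traces on Visibility from the character's location along the camera's forward vector, draws it for debugging, and applies damage to the hit actor.
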(event Input|EnhancedActionEvents|EnhancedInputActionIA_Shoot
  (params (ActionValue :type Boolean) (ElapsedSeconds :type Float%20%28double-precision%29) (TriggeredSeconds :type Float%20%28double-precision%29) (InputAction :type Input%20Action%20Object%20Reference :default "/Game/FirstPerson/Input/Actions/IA_Shoot.IA_Shoot"))
  (bind _as_bp_first_person_character (Variables|Default|GetAs%20BP%20First%20Person%20Character))
  (bind _returnvalue (Transformation|GetActorLocation _as_bp_first_person_character))
  (bind _outhit (Collision|LineTraceByChannel _returnvalue (+ _returnvalue (* (Transformation|GetActorForwardVector (Game|GetPlayerCameraManager 0)) 1e+04)) "TraceTypeQuery1" false 0 "ForDuration"))
  (Game|Damage|ApplyDamage (.HitActor (Collision|BreakHitResult _outhit)) (Variables|Weapon|GetDamage) 0 (Variables|Default|GetAs%20BP%20First%20Person%20Character) "/Script/Engine.DamageType"))

(event EventBeginPlay
  (bind _asplayer (Utilities|Casting|CastToBP_FirstPersonCharacter (Components|GetOwner)))
  (bind _output_get (Variables|Default|SetAs%20BP%20First%20Person%20Character _asplayer))
  (bind _asplayer_controller (Utilities|Casting|CastToPlayerController (Pawn|GetController _output_get)))
  (Utilities|IsValid (PlayerController|LocalPlayerSubsystems|GetEnhancedInputLocalPlayerSubsystem _asplayer_controller)
    (:Is%20Valid
      (Input|AddMappingContext (PlayerController|LocalPlayerSubsystems|GetEnhancedInputLocalPlayerSubsystem _asplayer_controller) "/Game/FirstPerson/Input/IMC_Weapons.IMC_Weapons" 1 "(bIgnoreAllPressedKeysUntilRelease=True,bForceImmediately=False,bNotifyUserSettings=False)"))))

(event EventTick
  (params (DeltaSeconds :type Float%20%28single-precision%29)))