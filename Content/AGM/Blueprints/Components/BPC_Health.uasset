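; BPC_Health is a health component that takes damage and broadcasts death.
; A damage event subtracts from CurrentHealth, or, on a lethal hit, calls OnDeath with the causer and itself, leaving health unchanged.
; A separate custom event binds an OnDeath handler that, if the causer has the "Tagged" tag, clears all the causer's tags and adds "None" to this component's tags.
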(event Custom|CustomEvent_0
  (params (DamageCauser :type Object%20Object%20Reference) (DamagedPlayer :type Object%20Object%20Reference))
  (for _array_element (Variables|/Script/Engine.Actor|GetTags (Variables|Default|GetDamage%20Causer))
    (if (== _array_element "Tagged")
      (Utilities|Array|Clear (Variables|/Script/Engine.Actor|GetTags (Variables|Default|GetDamage%20Causer)))
      (Utilities|Array|Add (Variables|Default|GetComponentTags) ""))))

(event Custom|CustomEvent
  (EventDispatchers|BindEventtoOnDeath (delegate Custom|CustomEvent_0)))

(event Custom|CustomEvent_1
  (params (Damage :type Float%20%28single-precision%29) (DamageType :type Damage%20Type%20Object%20Reference) (InstigatedBy :type Controller%20Object%20Reference) (DamageCauser :type Actor%20Object%20Reference))
  (bind _self self)
  (Variables|Default|SetDamage%20Causer DamageCauser)
  (if (<= (- (Variables|Default|GetCurrentHealth) Damage) 0.0)
    (Default|CallOnDeath _self (Variables|Default|GetDamage%20Causer) _self)
    (else
      (Variables|Default|SetCurrentHealth (- (Variables|Default|GetCurrentHealth) Damage)))))

(event EventTick
  (params (DeltaSeconds :type Float%20%28single-precision%29)))

(event EventBeginPlay)