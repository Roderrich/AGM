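; Shotgun component that gives the first-person player hitscan spread fire with ammo tracking.
; Triggered fires at once and starts a looping one-second timer, which Untriggered clears.
; Each shot casts debug-drawn line traces in a random cone from the camera, spending ammo and calling ApplyDamage per trace, with no damage amount set.
; Firing at exactly zero ammo instantly refills to maximum instead of shooting.
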(event Custom|Shoot
  (bind _as_player (Variables|Default|GetAs%20Player))
  (bind _firstpersoncamera (Variables|/Game/FirstPerson/Blueprints/BP_FirstPersonCharacter.BP_FirstPersonCharacter_C|GetFirstPersonCamera _as_player))
  (bind _returnvalue (Transformation|GetWorldLocation _firstpersoncamera))
  (if (== (Variables|Default|GetCurrentAmmo) 0)
    (CallFunction|Reload)
    (else
      (for _index (range 0 10)
        (bind _outhit (Collision|LineTraceByChannel _returnvalue (+ _returnvalue (* (Math|Random|RandomUnitVectorinConeinDegrees (Math|Vector|GetForwardVector _firstpersoncamera) 5.0) 1e+03)) "TraceTypeQuery1" false 0 "ForDuration"))
        (Math|Integer|DecrementInt (Variables|Default|GetCurrentAmmo)
          (:%20%20
            (Game|Damage|ApplyDamage (.HitActor (Collision|BreakHitResult _outhit)) 0.0 0 (Variables|Default|GetAs%20Player) "/Script/Engine.DamageType")))))))

(event Custom|Reload
  (Variables|Default|SetCurrentAmmo (Variables|Default|GetMaxAmmo)))

(event Custom|Untriggered
  (Utilities|Time|ClearandInvalidateTimerbyHandle (Variables|Default|GetFireTimer)))

(event Custom|Triggered
  (bind _returnvalue (Utilities|Time|SetTimerbyEvent (EventDispatchers|CreateEvent :!event Custom|Shoot) (/ 6e+01 6e+01) true))
  (Variables|Default|SetFireTimer _returnvalue)
  (CallFunction|Shoot))

(event EventBeginPlay
  (bind _asplayer (Utilities|Casting|CastToBP_FirstPersonCharacter (Game|GetPlayerCharacter 0)))
  (Variables|Default|SetAs%20Player _asplayer))

(event EventTick
  (params (DeltaSeconds :type Float%20%28single-precision%29)))