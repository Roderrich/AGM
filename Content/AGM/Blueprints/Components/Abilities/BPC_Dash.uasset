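; BPC_Dash is a dash ability component that launches the character along a supplied forward vector when activated.
; On the ground it first applies a small upward launch and waits one tick before dashing, while a falling character dashes immediately.
; Each dash turns on the first-person camera's post-process blend, and a short timer clears it through a single FInterpTo call rather than a per-frame fade.
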(event Custom|ActivateAbility
  (params (ForwardVector :type Vector) (ID :type BP%20First%20Person%20Character%20Object%20Reference))
  (Variables|Default|SetID ID)
  (if (AI|Components|NavMovement|IsFalling (Variables|/Script/Engine.Character|GetCharacterMovement (Variables|Default|GetID)))
    (Character|LaunchCharacter (Variables|Default|GetID) (* ForwardVector 1.5e+03) false false)
    (CallFunction|VFX)
    (else
      (Character|LaunchCharacter (Variables|Default|GetID) "0.000000,0.000000,100.000000" false false)
      (Utilities|FlowControl|DelayUntilNextTick)
      (Character|LaunchCharacter (Variables|Default|GetID) (* ForwardVector 1.5e+03) false false)
      (CallFunction|VFX))))

(event Custom|VFX
  (Class|CameraComponent|SetPostProcessBlendWeight (Variables|/Game/FirstPerson/Blueprints/BP_FirstPersonCharacter.BP_FirstPersonCharacter_C|GetFirstPersonCamera (Variables|Default|GetID)) 1.0)
  (Utilities|Time|SetTimerbyEvent (delegate Custom|Clear%20VFX) 0.5))

(event Custom|Clear%20VFX
  (Class|CameraComponent|SetPostProcessBlendWeight (Variables|/Game/FirstPerson/Blueprints/BP_FirstPersonCharacter.BP_FirstPersonCharacter_C|GetFirstPersonCamera (Variables|Default|GetID)) (Math|Interpolation|FInterpTo 1.0 0.0 1.0 1.0)))

(event EventTick
  (params (DeltaSeconds :type Float%20%28single-precision%29)))