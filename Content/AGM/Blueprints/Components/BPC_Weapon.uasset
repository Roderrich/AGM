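; Weapon component for the first-person player that loads per-weapon stats from DT_Weapon on BeginPlay.
; Trigger events either start a looping fire-rate timer for automatic weapons or fire single shots gated by a cooldown timer.
; Shoot spends ammo on a debug-drawn camera line trace and applies damage, while Reload refills instantly.
; ActivateAbility is empty, and leftover ability and warp-dash logic is mostly disconnected.
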(event Custom|Launch
  (bind _as_bp_first_person_character (Variables|Default|GetAs%20BP%20First%20Person%20Character))
  (bind _rootcomponent (Variables|/Script/Engine.Actor|GetRootComponent _as_bp_first_person_character))
  ;[0.15 0.15 0.15 0.5] Warp
  (if (not (Utilities|Operators|EqualEqual (Variables|Default|GetNewVar_0) (Variables|Default|GetDashLocation) 1e+02))
    (Transformation|SetWorldLocation _rootcomponent (+ (Transformation|GetWorldLocation _rootcomponent) (* (Math|Vector|GetForwardVector (Variables|/Game/FirstPerson/Blueprints/BP_FirstPersonCharacter.BP_FirstPersonCharacter_C|GetFirstPersonCamera _as_bp_first_person_character)) 1e+03)) false false)))

(event Custom|ActivateAbility
  (params (ID :type Integer))
  ;[0.15 0.15 0.15 0.5] Abilities
)

(event Custom|Reload
  (Variables|Weapon|SetCurrentAmmo (Variables|Weapon|GetMaxAmmo)))

(event Custom|Shoot
  (bind _as_bp_first_person_character (Variables|Default|GetAs%20BP%20First%20Person%20Character))
  (bind _firstpersoncamera (Variables|/Game/FirstPerson/Blueprints/BP_FirstPersonCharacter.BP_FirstPersonCharacter_C|GetFirstPersonCamera _as_bp_first_person_character))
  (bind _returnvalue (Transformation|GetWorldLocation _firstpersoncamera))
  (bind _returnvalue_2 (Utilities|Time|SetTimerbyEvent (delegate Custom|CustomEvent) (/ 6e+01 (Variables|Weapon|GetFireRate))))
  (Variables|Default|SetCooldownTimer _returnvalue_2)
  (if (not (== (Variables|Weapon|GetCurrentAmmo) 0))
    (bind _outhit (Collision|LineTraceByChannel _returnvalue (+ _returnvalue (* (Math|Vector|GetForwardVector _firstpersoncamera) 1e+04)) "TraceTypeQuery1" false 0 "ForDuration"))
    (Math|Integer|DecrementInt (Variables|Weapon|GetCurrentAmmo)
      (:%20%20
        (Game|Damage|ApplyDamage (.HitActor (Collision|BreakHitResult _outhit)) (Variables|Weapon|GetDamage) 0 (Variables|Default|GetAs%20BP%20First%20Person%20Character) "/Script/Engine.DamageType")))))

(event Custom|Untriggered
  (Utilities|Time|ClearandInvalidateTimerbyHandle (Variables|Default|GetAutomaticFireTimer)))

(event Custom|Triggered
  (if (Variables|Default|GetWLoop)
    (bind _returnvalue (Utilities|Time|SetTimerbyEvent (EventDispatchers|CreateEvent :!event Custom|Shoot) (/ 6e+01 (Variables|Weapon|GetFireRate)) true))
    (Variables|Default|SetAutomaticFireTimer _returnvalue)
    (CallFunction|Shoot)
    (elif (not (Utilities|Time|IsValidTimerHandle (Variables|Default|GetCooldownTimer)))
      (CallFunction|Shoot))))

(event Custom|CustomEvent
  (Utilities|Time|ClearandInvalidateTimerbyHandle (Variables|Default|GetCooldownTimer)))

(event EventBeginPlay
  (bind _asplayer (Utilities|Casting|CastToBP_FirstPersonCharacter (Game|GetPlayerCharacter 0)))
  (Variables|Default|SetAs%20BP%20First%20Person%20Character _asplayer)
  (bind _returnvalue (Utilities|GetDataTableRow "/Game/AGM/Blueprints/Weapons/DT_Weapon.DT_Weapon" (Utilities|Select :Index (Variables|Default|GetEnum) :NewEnumerator0 "Pistol" :NewEnumerator1 "Revolver" :NewEnumerator2 "SMG" :NewEnumerator3 "Shotgun" :NewEnumerator4 "AssaultRifle" :NewEnumerator5 "MarksmanRifle"))
    (:then
      (Variables|Weapon|SetWeapon%20Type (.WeaponType (Utilities|Struct|BreakS_Weapon _returnvalue)))
      (Variables|Weapon|SetFireRate (.FireRate (Utilities|Struct|BreakS_Weapon _returnvalue)))
      (bind _output_get (Variables|Weapon|SetMaxAmmo (.MaxAmmo (Utilities|Struct|BreakS_Weapon _returnvalue))))
      (Variables|Weapon|SetCurrentAmmo _output_get)
      (Variables|Weapon|SetDamage (.Damage (Utilities|Struct|BreakS_Weapon _returnvalue)))
      (Variables|Weapon|SetCooldown (.Cooldown (Utilities|Struct|BreakS_Weapon _returnvalue)))
      (Variables|Default|SetWLoop (.AutoFire (Utilities|Struct|BreakS_Weapon _returnvalue))))
    (:RowNotFound
      (Development|PrintString "ROW NOT FOUND"))))

(event EventTick
  (params (DeltaSeconds :type Float%20%28single-precision%29)))