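; Actor that builds an ice shape at runtime in a dynamic mesh from Niagara particle data.
; On BeginPlay it spawns NS_IcicleData at its location and passes itself as the system's export callback object.
; Each exported particle's position and size append a Geometry Script sphere box to the DynamicMeshComponent, offset relative to the actor's location.
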(event Custom|CustomEvent_0
  (params (Location :type Vector) (Size :type Float%20%28double-precision%29))
  (bind _returnvalue (DynamicMeshComponent|GetDynamicMesh (Variables|DynamicMeshActor|GetDynamicMeshComponent)))
  (Class|GeometryScriptLibraryMeshPrimitiveFunctions|AppendSphereBox :TargetMesh _returnvalue :Transform (Math|Conversions|ToTransform(Vector) (- Location (Transformation|GetActorLocation))) :Radius Size :Debug 0))

(event EventBeginPlay
  (bind _returnvalue (Niagara|SpawnSystematLocation "/Game/AGM/VFX/NS_IcicleData.NS_IcicleData" (Transformation|GetActorLocation)))
  (bind _output_get (Variables|Default|SetNewVar _returnvalue))
  (Niagara|SetNiagaraVariable(Object) _output_get "Object" self))

(event Collision|EventActorBeginOverlap
  (params (OtherActor :type Actor%20Object%20Reference)))

(event EventTick
  (params (DeltaSeconds :type Float%20%28single-precision%29)))

(event EventParticleData
  (params (Data :type Array%20of%20Basic%20Particle%20Data%20Structures) (NiagaraSystem :type Niagara%20System%20Object%20Reference) (SimulationPositionOffset :type Vector%20%28by%20ref%29 :default "0, 0, 0"))
  (for _array_element Data
    (CallFunction|CustomEvent0 (.Position (Utilities|Struct|BreakBasicParticleData _array_element)) (.Size (Utilities|Struct|BreakBasicParticleData _array_element)))))

(fn ConstructionScript)