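; BP_Ice1 is an ice VFX actor that turns a Niagara icicle burst into dynamic mesh geometry with collision.
; On BeginPlay it spawns NS_IcicleBurst and passes itself as the particle export callback, storing received positions as transforms.
; When the system finishes, Geometry Script sweeps scaled triangular profiles between seven pairs of stored points, recomputing normals and regenerating simple collision after each sweep.
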(event Custom|CallSweep
  (params (PSystem :type Niagara%20Component%20Object%20Reference))
  (bind _transform (Variables|Default|GetTransform))
  (bind _returnvalue (DynamicMeshComponent|GetDynamicMesh (Variables|DynamicMeshActor|GetDynamicMeshComponent)))
  (for _index (range 0 6)
    (bind _returnvalue_2 (Class|GeometryScriptLibraryMeshPrimitiveFunctions|AppendSweepPolygon :TargetMesh _returnvalue :PolygonVertices (Utilities|Array|MakeArray "(X=1.000000,Y=0.000000)" "(X=0.000000,Y=1.000000)" "(X=-1.000000,Y=0.000000)") :SweepPath (Utilities|Array|MakeArray (Utilities|Array|Get(acopy) _transform (* _index 2)) (Utilities|Array|Get(acopy) _transform (+ (* _index 2) 15))) :StartScale 5e+01 :Debug 0))
    (bind _returnvalue_3 (GeometryScript|Normals|RecomputeNormals :TargetMesh _returnvalue_2 :Debug 0))
    (bind _returnvalue_4 (Class|GeometryScriptLibraryCollisionFunctions|GenerateCollisionfromMesh :FromDynamicMesh _returnvalue_3 :Debug 0))
    (Class|GeometryScriptLibraryCollisionFunctions|SetSimpleCollisionOfDynamicMeshComponent :SimpleCollision _returnvalue_4 :DynamicMeshComponent (Variables|DynamicMeshActor|GetDynamicMeshComponent) :Debug 0)))

(event EventBeginPlay
  (bind _returnvalue (Niagara|SpawnSystematLocation "/Game/AGM/VFX/NS_IcicleBurst.NS_IcicleBurst" (Transformation|GetActorLocation) (Transformation|GetActorRotation)))
  (bind _output_get (Variables|Default|SetNewVar _returnvalue))
  (Niagara|SetNiagaraVariable(Object) _output_get "Object" self)
  (EventDispatchers|BindEventtoOnSystemFinished _returnvalue (delegate Custom|CallSweep)))

(event Collision|EventActorBeginOverlap
  (params (OtherActor :type Actor%20Object%20Reference)))

(event EventTick
  (params (DeltaSeconds :type Float%20%28single-precision%29)))

(event EventParticleData
  (params (Data :type Array%20of%20Basic%20Particle%20Data%20Structures) (NiagaraSystem :type Niagara%20System%20Object%20Reference) (SimulationPositionOffset :type Vector%20%28by%20ref%29 :default "0, 0, 0"))
  (for _array_element Data
    (bind _returnvalue (Utilities|Array|Add (Variables|Default|GetTransform) (Math|Conversions|ToTransform(Vector) (.Position (Utilities|Struct|BreakBasicParticleData _array_element)))))))

(fn ConstructionScript)