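; BP_PC is a player controller that sets up the local player's input and main screen UI at the start of play.
; BeginPlay retries on a short delay until a pawn is possessed, caches it as a BP_FirstPersonCharacter, then adds the default Enhanced Input mapping context.
; SwitchWidgets creates WBP_MainScreen and picks its widget switcher page by hard-coded level name, with a fallback page, before it is added to the player's screen.
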(event Custom|CustomEvent)

(event Custom|AssignPlayerID)

(event Input|EnhancedActionEvents|EnhancedInputActionIA_Ability
  (params (ActionValue :type Boolean) (ElapsedSeconds :type Float%20%28double-precision%29) (TriggeredSeconds :type Float%20%28double-precision%29) (InputAction :type Input%20Action%20Object%20Reference :default "/Game/FirstPerson/Input/Actions/IA_Ability.IA_Ability")))

(event EventBeginPlay
  (bind _returnvalue (Pawn|GetControlledPawn))
  (bind _self self)
  (bind _returnvalue_2 (PlayerController|LocalPlayerSubsystems|GetEnhancedInputLocalPlayerSubsystem _self))
  (Utilities|IsValid _returnvalue :!label _label
    (:Is%20Valid
      (bind _asplayer (Utilities|Casting|CastToBP_FirstPersonCharacter _returnvalue))
      (Variables|Default|SetAs%20Player _asplayer)
      (Utilities|IsValid _returnvalue_2
        (:Is%20Valid
          (Input|AddMappingContext _returnvalue_2 "/Game/FirstPerson/Input/IMC_Default.IMC_Default" 0 "(bIgnoreAllPressedKeysUntilRelease=True,bForceImmediately=False,bNotifyUserSettings=False)")
          (bind _widget (CallFunction|SwitchWidgets))
          (UserInterface|Viewport|AddtoPlayerScreen _widget))))
    (:Is%20Not%20Valid
      (Utilities|FlowControl|Delay 0.2)
      (goto _label))))

(event EventTick
  (params (DeltaSeconds :type Float%20%28single-precision%29)))

(fn ConstructionScript)

(fn SwitchWidgets
  (bind _returnvalue (UserInterface|CreateWidget "/Game/AGM/UI/WBP_MainScreen.WBP_MainScreen_C" self))
  (Variables|Default|SetWidget _returnvalue)
  (bind _returnvalue_2 (Game|GetCurrentLevelName true))
  (if (Utilities|Enum|Equal(Enum) _returnvalue_2 "L_Tutorial")
    (Variables|/Script/UMG.WidgetSwitcher|SetActiveWidgetIndex (Variables|/Game/AGM/UI/WBP_MainScreen.WBP_MainScreen_C|GetWidgetSwitcher_0 (Variables|Default|GetWidget)) 1)
    (return (Variables|Default|GetWidget))
    (else
      (bind _returnvalue_3 (Game|GetCurrentLevelName true))
      (if (Utilities|Enum|Equal(Enum) _returnvalue_3 "FirstPersonMap")
        (Variables|/Script/UMG.WidgetSwitcher|SetActiveWidgetIndex (Variables|/Game/AGM/UI/WBP_MainScreen.WBP_MainScreen_C|GetWidgetSwitcher_0 (Variables|Default|GetWidget)) 0)
        (return (Variables|Default|GetWidget))
        (else
          (bind _returnvalue_4 (Game|GetCurrentLevelName true))
          (if (Utilities|Enum|Equal(Enum) _returnvalue_4 "L_Arena")
            (Variables|/Script/UMG.WidgetSwitcher|SetActiveWidgetIndex (Variables|/Game/AGM/UI/WBP_MainScreen.WBP_MainScreen_C|GetWidgetSwitcher_0 (Variables|Default|GetWidget)) 1)
            (return (Variables|Default|GetWidget))
            (else
              (bind _returnvalue_5 (Game|GetCurrentLevelName true))
              (if (Utilities|Enum|Equal(Enum) _returnvalue_5 "L_MiniArena")
                (Variables|/Script/UMG.WidgetSwitcher|SetActiveWidgetIndex (Variables|/Game/AGM/UI/WBP_MainScreen.WBP_MainScreen_C|GetWidgetSwitcher_0 (Variables|Default|GetWidget)) 0)
                (return (Variables|Default|GetWidget))
                (else
                  (Variables|/Script/UMG.WidgetSwitcher|SetActiveWidgetIndex (Variables|/Game/AGM/UI/WBP_MainScreen.WBP_MainScreen_C|GetWidgetSwitcher_0 (Variables|Default|GetWidget)) 5)
                  (return (Variables|Default|GetWidget)))))))))))