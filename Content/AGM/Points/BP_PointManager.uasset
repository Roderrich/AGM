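; BP_PointManager keeps up to about ten point pickups active in the level by recycling pre-placed BP_Points actors as a pool.
; On BeginPlay it gathers every BP_Points, binds their pickup events to decrement the spawned count, and starts a looping one-second timer.
; Each tick of that timer below the cap claims an unused point and moves it to a random, slightly raised navigable location on the RecastNavMesh.
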(event Custom|Spawn
  (if (< (Variables|Default|GetPointsSpawned) 10)
    (bind _output (CallFunction|GetPoints))
    (bind _outactors (Actor|GetAllActorsOfClass "/Script/NavigationSystem.RecastNavMesh"))
    (for _array_element _outactors
      (bind _randomlocation (Class|NavigationSystemV1|GetRandomLocationinNavigableRadius (Variables|Default|GetOrigin) 2e+04 _array_element 0))
      (Transformation|SetActorLocation _output (+ _randomlocation "0.000000,0.000000,100.000000") false false)
      (Math|Integer|IncrementInt (Variables|Default|GetPointsSpawned)))))

(event Custom|StartSpawn
  (Utilities|Time|SetTimerbyEvent (delegate Custom|Spawn) 1.0 true))

(event Custom|PointGain
  (Math|Integer|DecrementInt (Variables|Default|GetPointsSpawned)))

(event EventBeginPlay
  (bind _outactors (Actor|GetAllActorsOfClass "/Game/AGM/Points/BP_Points.BP_Points_C"))
  (bind _output_get (Variables|Default|SetPoints _outactors))
  (CallFunction|StartSpawn)
  (EventDispatchers|BindEventtoPickuped _output_get (delegate Custom|PointGain)))

(event Collision|EventActorBeginOverlap
  (params (OtherActor :type Actor%20Object%20Reference)))

(event EventTick
  (params (DeltaSeconds :type Float%20%28single-precision%29)))

(fn ConstructionScript)

(fn CheckinUse)

(fn GetPoints
  (for (_array_element _array_index) (Variables|Default|GetPoints)
    (bind _use (Class|BPIPOINT|CheckUse(Message) _array_element))
    (if (not _use)
      (Class|BPIPOINT|SetinUse(Message) (Utilities|Array|Get(acopy) (Variables|Default|GetPoints) _array_index))
      (bind _output_get (LocalVariables|SetNewLocalVar (Utilities|Array|Get(acopy) (Variables|Default|GetPoints) _array_index)))
      (return _output_get))))